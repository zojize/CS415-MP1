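; BP_Enemy is an enemy actor that moves in discrete steps and damages the player on contact.
; BeginPlay picks a random X/Z direction and starts a looping one-second timer that offsets the actor along it and counts steps.
; Box overlap with BP_Player removes a hit point, refreshes the display, destroys the enemy, and shows restart at zero or below.
; A MovePattern switch exists in MoveByPattern but never runs.
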(event OnComponentBeginOverlap(Box)
  (params (OverlappedComponent :type Primitive%20Component%20Object%20Reference) (OtherActor :type Actor%20Object%20Reference) (OtherComp :type Primitive%20Component%20Object%20Reference) (OtherBodyIndex :type Integer) (bFromSweep :type Boolean) (SweepResult :type Hit%20Result%20Structure%20%28by%20ref%29))
  (bind _asbp_player (Utilities|Casting|CastToBP_Player OtherActor))
  (bind _result (Math|Integer|DecrementInt (Variables|/Game/InfiniteMatrix/Blueprints/BP_Player.BP_Player_C|GetHitPoints _asbp_player))
    (:%20%20
      (Default|UpdateHitPoints _asbp_player)
      (Actor|DestroyActor)
      (if (<= _result 0)
        (Default|DisplayRestart _asbp_player)))))

(event Custom|Move
  (CallFunction|MovebyPattern)
  (Math|Integer|IncrementInt (Variables|Default|GetSteps)))

(event EventBeginPlay
  (bind _returnvalue (Math|Random|RandomUnitVector))
  (bind _returnvalue_2 (* _returnvalue 5.0))
  (Utilities|Time|SetTimerbyFunctionName 0 "Move" 1.0 true)
  (Variables|Default|SetDirection (Math|Vector|MakeVector (.x _returnvalue_2) 0.0 (.z _returnvalue_2))))

(event Collision|EventActorBeginOverlap
  (params (OtherActor :type Actor%20Object%20Reference)))

(event EventTick
  (params (DeltaSeconds :type Float%20%28single-precision%29)))

(fn ConstructionScript)

(fn MovebyPattern
  (Transformation|AddActorLocalOffset (Variables|Default|GetDirection) false false))