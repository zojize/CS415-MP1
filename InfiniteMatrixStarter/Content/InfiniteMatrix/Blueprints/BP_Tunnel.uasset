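; BP_Tunnel is an endless-runner tunnel segment with a spinning holed wall, a score collider and a heart pickup.
; Overlapping TriggerZone makes TunnelSpawner spawn the next segment, then this one self-destructs after a short delay.
; Wall hits cost BP_Player health once; clean passes add score and speed, and hearts restore limited health.
; Exposed functions randomize wall mesh and roll, offset the heart or remove it.
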(event OnComponentBeginOverlap(TriggerZone)
  (params (OverlappedComponent :type Primitive%20Component%20Object%20Reference) (OtherActor :type Actor%20Object%20Reference) (OtherComp :type Primitive%20Component%20Object%20Reference) (OtherBodyIndex :type Integer) (bFromSweep :type Boolean) (SweepResult :type Hit%20Result%20Structure%20%28by%20ref%29))
  (Utilities|Casting|CastToBP_Player OtherActor)
  (Default|SpawnTunnelatSpawnPoint (Variables|Default|GetTunnelSpawner))
  (Utilities|FlowControl|Delay 0.5)
  (Actor|DestroyActor))

(event OnComponentBeginOverlap(WallMesh)
  (params (OverlappedComponent :type Primitive%20Component%20Object%20Reference) (OtherActor :type Actor%20Object%20Reference) (OtherComp :type Primitive%20Component%20Object%20Reference) (OtherBodyIndex :type Integer) (bFromSweep :type Boolean) (SweepResult :type Hit%20Result%20Structure%20%28by%20ref%29))
  (if (not (Variables|Default|GetHitWall))
    (bind _asbp_player (Utilities|Casting|CastToBP_Player OtherActor))
    (Variables|Default|SetHitWall true)
    (bind _result (Math|Integer|DecrementInt (Variables|/Game/InfiniteMatrix/Blueprints/BP_Player.BP_Player_C|GetHitPoints _asbp_player))
      (:%20%20
        (Default|UpdateHitPoints _asbp_player)
        (if (<= _result 0)
          (Default|DisplayRestart _asbp_player))))))

(event OnComponentBeginOverlap(Heart)
  (params (OverlappedComponent :type Primitive%20Component%20Object%20Reference) (OtherActor :type Actor%20Object%20Reference) (OtherComp :type Primitive%20Component%20Object%20Reference) (OtherBodyIndex :type Integer) (bFromSweep :type Boolean) (SweepResult :type Hit%20Result%20Structure%20%28by%20ref%29))
  (if (not (Variables|Default|GetHitWall))
    (bind _asbp_player (Utilities|Casting|CastToBP_Player OtherActor))
    (if (<= (Variables|/Game/InfiniteMatrix/Blueprints/BP_Player.BP_Player_C|GetHitPoints _asbp_player) 4)
      (Math|Integer|IncrementInt (Variables|/Game/InfiniteMatrix/Blueprints/BP_Player.BP_Player_C|GetHitPoints _asbp_player)
        (:%20%20
          (Default|UpdateHitPoints _asbp_player)
          (Components|DestroyComponent (Variables|Default|GetHeart)))))))

(event OnComponentBeginOverlap(ScoreCollider)
  (params (OverlappedComponent :type Primitive%20Component%20Object%20Reference) (OtherActor :type Actor%20Object%20Reference) (OtherComp :type Primitive%20Component%20Object%20Reference) (OtherBodyIndex :type Integer) (bFromSweep :type Boolean) (SweepResult :type Hit%20Result%20Structure%20%28by%20ref%29))
  (if (not (Variables|Default|GetHitWall))
    (bind _asbp_player (Utilities|Casting|CastToBP_Player OtherActor))
    (Math|Integer|IncrementInt (Variables|/Game/InfiniteMatrix/Blueprints/BP_Player.BP_Player_C|GetScore _asbp_player)
      (:%20%20
        (Default|UpdateScore _asbp_player)
        (Variables|/Game/InfiniteMatrix/Blueprints/BP_Player.BP_Player_C|SetForwardSpeed%20 _asbp_player (+ (Variables|/Game/InfiniteMatrix/Blueprints/BP_Player.BP_Player_C|GetForwardSpeed%20 _asbp_player) 2e+01))))))

(event EventBeginPlay)

(event EventTick
  (params (DeltaSeconds :type Float%20%28single-precision%29))
  (Transformation|AddLocalRotation (Variables|Default|GetWallMesh) (Math|Rotator|MakeRotator (* DeltaSeconds (Variables|Default|GetRotateSpeed)) 0.0 0.0) false false))

(fn ConstructionScript)

(fn RandomizeWall
  (Components|StaticMesh|SetStaticMesh (Variables|Default|GetWallMesh) (Utilities|Select :Index (Math|Random|RandomIntegerinRange 0 3) :Option%200 "/Game/InfiniteMatrix/Meshes/SM_Hole_01.SM_Hole_01" :Option%201 "/Game/InfiniteMatrix/Meshes/SM_Hole_02.SM_Hole_02" :Option%202 "/Game/InfiniteMatrix/Meshes/SM_Hole_03.SM_Hole_03" :Option%203 "/Game/InfiniteMatrix/Meshes/SM_Hole_04.SM_Hole_04"))
  (Transformation|AddLocalRotation (Variables|Default|GetWallMesh) (Math|Rotator|MakeRotator (Math|Random|RandomFloatinRange 0.0 3.6e+02) 0.0 0.0) false false))

(fn RandomizeHeart
  (bind _returnvalue (Math|Random|RandomFloatinRange 0.0 3.6e+02))
  (bind _returnvalue_2 (Math|Random|RandomFloatinRange 0.0 4e+02))
  (Class|SceneComponent|AddLocalTransform (Variables|Default|GetHeart) (Math|Transform|MakeTransform (Math|Vector|MakeVector (* (Math|Trig|Cos(Degrees) _returnvalue) _returnvalue_2) (* (Math|Trig|Sin(Degrees) _returnvalue) _returnvalue_2) 0.0) "0, 0, 0" "1.000000,1.000000,1.000000") false false))

(fn DestroyHeart
  (Components|DestroyComponent (Variables|Default|GetHeart)))