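; BP_Bullet is the player's projectile, flying forward along world X to destroy enemies and add to the score.
; On spawn it sets its speed to triple the player's forward speed, then moves each tick and expires after five seconds.
; Sphere overlaps destroy it on tunnel walls, or destroy it along with a hit enemy and increment the player's score.
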(event OnComponentBeginOverlap(Sphere)
  (params (OverlappedComponent :type Primitive%20Component%20Object%20Reference) (OtherActor :type Actor%20Object%20Reference) (OtherComp :type Primitive%20Component%20Object%20Reference) (OtherBodyIndex :type Integer) (bFromSweep :type Boolean) (SweepResult :type Hit%20Result%20Structure%20%28by%20ref%29))
  (bind _asbp_tunnel (Utilities|Casting|CastToBP_Tunnel OtherActor)
    (:then
      (if (== OtherComp (Variables|/Game/InfiniteMatrix/Blueprints/BP_Tunnel.BP_Tunnel_C|GetWallMesh _asbp_tunnel))
        (Actor|DestroyActor)))
    (:CastFailed
      (bind _asbp_enemy (Utilities|Casting|CastToBP_Enemy OtherActor))
      (Actor|DestroyActor _asbp_enemy)
      (Actor|DestroyActor)
      (bind _outactors (Actor|GetAllActorsOfClass "/Game/InfiniteMatrix/Blueprints/BP_Player.BP_Player_C"))
      (Math|Integer|IncrementInt (Variables|/Game/InfiniteMatrix/Blueprints/BP_Player.BP_Player_C|GetScore (Utilities|Array|Get(acopy) _outactors))
        (:%20%20
          (Default|UpdateScore (Utilities|Array|Get(acopy) _outactors)))))))

(event EventBeginPlay
  (bind _outactors (Actor|GetAllActorsOfClass "/Game/InfiniteMatrix/Blueprints/BP_Player.BP_Player_C"))
  (Variables|Default|SetForwardSpeed (* (Variables|/Game/InfiniteMatrix/Blueprints/BP_Player.BP_Player_C|GetForwardSpeed%20 (Utilities|Array|Get(acopy) _outactors)) 3.0)))

(event EventTick
  (params (DeltaSeconds :type Float%20%28single-precision%29))
  (if (>= (Variables|Default|GetAge) 5.0)
    (Actor|DestroyActor)
    (else
      (Variables|Default|SetAge (+ DeltaSeconds (Variables|Default|GetAge)))
      (Transformation|AddActorWorldOffset (Math|Vector|MakeVector (* DeltaSeconds (Variables|Default|GetForwardSpeed)) 0.0 0.0)))))

(fn ConstructionScript)